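; Player controller that turns player input into movement, jumping and looking for the first-person FP_Character it possesses.
; Each input event casts the controlled pawn to FP_Character and does nothing if the cast fails.
; Movement axes use only the control rotation's yaw for forward and right directions, keeping movement independent of camera pitch.
; Mouse and gamepad look axes feed pitch and yaw input unscaled, and jump press and release start and stop jumping.
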(event Input|ActionEvents|InputActionJump
  (params (Key :type Key%20Structure :default "None"))
  (:Pressed
    (bind _asfp_character (Utilities|Casting|CastToFP_Character (Pawn|GetControlledPawn)))
    (Character|Jump _asfp_character))
  (:Released
    (bind _asfp_character_2 (Utilities|Casting|CastToFP_Character (Pawn|GetControlledPawn)))
    (Character|StopJumping _asfp_character_2)))

(event Input|AxisEvents|InputAxisMoveForward/Backward
  (params (AxisValue :type Float%20%28single-precision%29))
  (bind _asfp_character (Utilities|Casting|CastToFP_Character (Pawn|GetControlledPawn)))
  (Pawn|Input|AddMovementInput _asfp_character (Math|Vector|GetForwardVector (Math|Rotator|MakeRotator 0.0 0.0 (.Yaw (Math|Rotator|BreakRotator (Pawn|GetControlRotation :!class /Script/Engine.Controller))))) AxisValue false))

(event Input|AxisEvents|InputAxisMoveRight/Left
  (params (AxisValue :type Float%20%28single-precision%29))
  (bind _asfp_character (Utilities|Casting|CastToFP_Character (Pawn|GetControlledPawn)))
  (Pawn|Input|AddMovementInput _asfp_character (Math|Vector|GetRightVector (Math|Rotator|MakeRotator 0.0 0.0 (.Yaw (Math|Rotator|BreakRotator (Pawn|GetControlRotation :!class /Script/Engine.Controller))))) AxisValue false))

(event Input|AxisEvents|InputAxisLookUp/DownGamepad
  (params (AxisValue :type Float%20%28single-precision%29))
  (bind _asfp_character (Utilities|Casting|CastToFP_Character (Pawn|GetControlledPawn)))
  (Pawn|Input|AddControllerPitchInput _asfp_character AxisValue))

(event Input|AxisEvents|InputAxisLookUp/DownMouse
  (params (AxisValue :type Float%20%28single-precision%29))
  (bind _asfp_character (Utilities|Casting|CastToFP_Character (Pawn|GetControlledPawn)))
  (Pawn|Input|AddControllerPitchInput _asfp_character AxisValue))

(event Input|AxisEvents|InputAxisTurnRight/LeftGamepad
  (params (AxisValue :type Float%20%28single-precision%29))
  (bind _asfp_character (Utilities|Casting|CastToFP_Character (Pawn|GetControlledPawn)))
  (Pawn|Input|AddControllerYawInput _asfp_character AxisValue))

(event Input|AxisEvents|InputAxisTurnRight/LeftMouse
  (params (AxisValue :type Float%20%28single-precision%29))
  (bind _asfp_character (Utilities|Casting|CastToFP_Character (Pawn|GetControlledPawn)))
  (Pawn|Input|AddControllerYawInput _asfp_character AxisValue))

(fn ConstructionScript)