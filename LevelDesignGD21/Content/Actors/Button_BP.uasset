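; Push-button actor that the first-person character uses to trigger a platform move, with two lights showing red or green.
; Box overlap drives Turn_On/Turn_Off prompt widgets and binding to the character's OnPush event, based on IsActivated and OneWay.
; A push on an activated one-way button deactivates it, turns the lights red and fires the MovePlatform dispatcher.
; Collapsed graphs handle prompts and light colors.
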(event OnComponentBeginOverlap(Box)
  (params (OverlappedComponent :type Primitive%20Component%20Object%20Reference) (OtherActor :type Actor%20Object%20Reference) (OtherComp :type Primitive%20Component%20Object%20Reference) (OtherBodyIndex :type Integer) (bFromSweep :type Boolean) (SweepResult :type Hit%20Result%20Structure%20%28by%20ref%29))
  (bind _asfp_character (Utilities|Casting|CastToFP_Character OtherActor))
  (if (Variables|Default|GetIsActivated)
    (if (Variables|Default|GetOneWay)
      (|Tutorial) ; enters at execute3
      (else
        (|Tutorial) ; enters at execute2
      ))
    (else
      (|Tutorial) ; enters at execute4
    )))

(event OnComponentEndOverlap(Box)
  (params (OverlappedComponent :type Primitive%20Component%20Object%20Reference) (OtherActor :type Actor%20Object%20Reference) (OtherComp :type Primitive%20Component%20Object%20Reference) (OtherBodyIndex :type Integer))
  (bind _asfp_character (Utilities|Casting|CastToFP_Character OtherActor))
  (|Tutorial
    (:then
      (EventDispatchers|BindEventtoOnPush (stale OnComponentBeginOverlap(Box) _asfp_character) (delegate Custom|MovePlatform) :!label _label))
    (:then2
      (EventDispatchers|UnbindEventfromOnPush _asfp_character (delegate Custom|MovePlatform)))
    (:then3
      (goto _label))))

(event Custom|MovePlatform
  (params (Push :type Boolean))
  (Viewport|RemoveAllWidgets)
  (if (Variables|Default|GetIsActivated)
    (if (Variables|Default|GetOneWay)
      (goto _label execute3)
      (else
        (|UIFixes :!label _label
          (:then
            _)
          (:then2
            _))
        (if Push
          (if (Variables|Default|GetIsActivated)
            (Variables|Default|SetIsActivated false)
            (|ChangeLightColor :!label _label_2
              (:then
                _)
              (:then2
                _))
            (Default|CallMovePlatform (Variables|Default|GetIsActivated))
            (else
              (Variables|Default|SetIsActivated true)
              (goto _label_2 execute2))))))
    (else
      (goto _label execute2))))

(event EventBeginPlay
  (Input|EnableInput (Game|GetPlayerController 0)))

(fn ConstructionScript)